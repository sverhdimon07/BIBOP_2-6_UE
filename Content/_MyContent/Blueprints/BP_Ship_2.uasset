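; Physics-driven ship that the player occupies through Interact and exits with a leave input, toggling its thruster and notifying BP_Player.
; Horizontal thrust input eases a strength value that drives engine audio RPM and, above a threshold, overrides forward velocity on Tick.
; Roll input applies yaw torque above that threshold; pitch, yaw and vertical thrust logic is unwired.
; BeginPlay shifts the center of mass toward the thruster in X and Y.
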(event `self.ReceiveBeginPlay`
  (bind _shipmodel (`self.ShipModel`))
  (bind (_returnvalue_x _returnvalue_y) (`KismetMathLibrary.BreakVector` (`KismetMathLibrary.GreaterGreater_VectorRotator` (- (`SceneComponent.K2_GetComponentLocation` (`self.PhysicsThruster`)) (`PrimitiveComponent.GetCenterOfMass` _shipmodel "None")) (`KismetMathLibrary.NegateRotator` (`SceneComponent.K2_GetComponentRotation` _shipmodel)))))
  ;[0.15 0 0 0.502] Initialization (очевидно, что метод инита не должен вызываться сам в данном ивенте, его должен вызывать бутстрап сцены)
  (`|ExecutionSequence`
    (:`then_0`
      (`PrimitiveComponent.SetCenterOfMass` _shipmodel (`KismetMathLibrary.MakeVector` _returnvalue_x _returnvalue_y) "None"))
    (:`then_1`
      ;[0.15 0 0 0.5] InitializationPlayer
      (bind _asbp_player (cast `/Game/_MyContent/Blueprints/BP_Player` (`GameplayStatics.GetPlayerCharacter` 0)))
      (set `self.Player` _asbp_player))
    (:`then_2`
      ;[0.15 0 0 0.5] InitializationStaticMeshComponent
      (set `self.StaticMesh` (`self.ShipModel`)))))

(event `self.Interact`
  (bind _player (`self.Player`))
  ;[0.15 0 0 0.502] Interaction (РАЗДЕЛИТЬ ЛОГИКУ ПОТОМ)
  (if (`self.IsShipOccupied`)
    (`KismetSystemLibrary.PrintString` "ALREADY OCCUPIED BY SOMEONE ELSE")
    (else
      (set `self.IsShipOccupied` true)
      (`KismetSystemLibrary.PrintString` "YOU ARE IN")
      (set `/Game/_MyContent/Blueprints/BP_Player.CurrentShip_2` self _player)
      (`/Game/_MyContent/Blueprints/BP_Player.Delegate OccupyShip_2` _player)
      (`ActorComponent.Activate` (`self.PhysicsThruster`) false))))

(event `EnhancedInput|/Game/_MyContent/InputActionContexts/ShipInputActions/IA_Leave`
  (params (ActionValue :type Boolean) (ElapsedSeconds :type "Float (double-precision)") (TriggeredSeconds :type "Float (double-precision)") (InputAction :type "InputAction Object Reference" :default "/Game/_MyContent/InputActionContexts/ShipInputActions/IA_Leave.IA_Leave"))
  (bind _player (`self.Player`))
  ;[0.15 0 0 0.502] Leaving
  (:`Started`
    (`KismetSystemLibrary.PrintString` "YOU ARE OUT")
    (`/Game/_MyContent/Blueprints/BP_Player.Delegate LeaveShip_2` _player)
    (set `self.IsShipOccupied` false)
    (set `/Game/_MyContent/Blueprints/BP_Player.CurrentShip_2` null _player)
    (`ActorComponent.Deactivate` (`self.PhysicsThruster`))))

(event `self.ReceiveTick`
  (params (DeltaSeconds :type "Float (single-precision)"))
  ;[0.15 0 0 0.5] GivingHorizontalThrust
  (if (>= (`self.HorizontalThrustStrength`) 300.0)
    (`PrimitiveComponent.SetPhysicsLinearVelocity` (`self.ShipModel`) (`self.RequiredHorizontalThrustDirection`) false "None")))

(event `EnhancedInput|/Game/_MyContent/InputActionContexts/ShipInputActions/IA_GiveHorizontalThrust`
  (params (ActionValue :type "Float (double-precision)") (ElapsedSeconds :type "Float (double-precision)") (TriggeredSeconds :type "Float (double-precision)") (InputAction :type "InputAction Object Reference" :default "/Game/_MyContent/InputActionContexts/ShipInputActions/IA_GiveHorizontalThrust.IA_GiveHorizontalThrust"))
  (bind _horizontalthruststrength (`self.HorizontalThrustStrength`))
  (bind _audiocurvesource (`self.AudioCurveSource`))
  ;[0.15 0 0 0.5] GivingHorizontalThrust
  (:`Triggered`
    (`|ExecutionSequence`
      (:`then_0`
        (if (>= ActionValue 0.0)
          (set `self.IncomingHorizontalThrustAlpha` 0.0)
          (else
            (set `self.IncomingHorizontalThrustAlpha` 1.0)))
        (bind _output_get (set `self.HorizontalThrustStrength` (`KismetMathLibrary.FInterpTo` _horizontalthruststrength (`KismetMathLibrary.Lerp` 0.0 (`self.MaxHorizontalThrustStrength`) (`self.IncomingHorizontalThrustAlpha`)) (`GameplayStatics.GetWorldDeltaSeconds`))))
        (`ActorComponent.Activate` _audiocurvesource false)
        (`AudioComponent.SetFloatParameter` _audiocurvesource "RPM" (`KismetMathLibrary.MapRangeClamped` (`KismetMathLibrary.Abs` _output_get) 0.0 5000.0 0.0 1.0)))
      (:`then_1`
        (set `self.RequiredHorizontalThrustDirection` (* (`SceneComponent.GetForwardVector` (`self.ShipModel`)) _horizontalthruststrength))))))

(event `EnhancedInput|/Game/_MyContent/InputActionContexts/ShipInputActions/IA_GiveVerticalThrust`
  (params (ActionValue :type "Float (double-precision)") (ElapsedSeconds :type "Float (double-precision)") (TriggeredSeconds :type "Float (double-precision)") (InputAction :type "InputAction Object Reference" :default "/Game/_MyContent/InputActionContexts/ShipInputActions/IA_GiveVerticalThrust.IA_GiveVerticalThrust"))
  ;[0.15 0 0 0.5] GivingVerticalThrust
)

(event `EnhancedInput|/Game/_MyContent/InputActionContexts/ShipInputActions/IA_Pitch`
  (params (ActionValue :type "Float (double-precision)") (ElapsedSeconds :type "Float (double-precision)") (TriggeredSeconds :type "Float (double-precision)") (InputAction :type "InputAction Object Reference" :default "/Game/_MyContent/InputActionContexts/ShipInputActions/IA_Pitch.IA_Pitch"))
  ;[0.15 0 0 0.5] RotationPitch
)

(event `EnhancedInput|/Game/_MyContent/InputActionContexts/ShipInputActions/IA_Yaw`
  (params (ActionValue :type "Float (double-precision)") (ElapsedSeconds :type "Float (double-precision)") (TriggeredSeconds :type "Float (double-precision)") (InputAction :type "InputAction Object Reference" :default "/Game/_MyContent/InputActionContexts/ShipInputActions/IA_Yaw.IA_Yaw"))
  ;[0.15 0 0 0.5] RotationYaw
)

(event `EnhancedInput|/Game/_MyContent/InputActionContexts/ShipInputActions/IA_Roll`
  (params (ActionValue :type "Float (double-precision)") (ElapsedSeconds :type "Float (double-precision)") (TriggeredSeconds :type "Float (double-precision)") (InputAction :type "InputAction Object Reference" :default "/Game/_MyContent/InputActionContexts/ShipInputActions/IA_Roll.IA_Roll"))
  ;[0.15 0 0 0.5] RotationRoll
  (:`Triggered`
    ;[0.15 0 0 0.5] RotationYaw
    (`self.Rotate` (`SceneComponent.GetUpVector` (`self.ShipModel`)) ActionValue (`self.YawStrength`))))

(fn `Rotate`
  (params (AddingRelativityDirection :type "Vector Structure") (Input :type "Float (double-precision)") (Strength :type "Float (double-precision)"))
  (if (>= (`self.HorizontalThrustStrength`) 300.0)
    (`PrimitiveComponent.AddTorqueInDegrees` (`self.ShipModel`) (* AddingRelativityDirection (* Input Strength)) "None" true)))

(fn `UserConstructionScript`)