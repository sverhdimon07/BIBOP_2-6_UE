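; BP_Bootstrap is a level bootstrap Blueprint that exposes a public event, DelegateReloadLevel, to reopen the current level by name.
; BeginPlay leads only to an empty sequence, so it performs no initialization.
; Disconnected leftover logic would spawn a PlayerStart according to the game instance's ModeNumber, through a cast with no target class, and restart BP_Player_2 at a player start.
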(event `self.ReceiveBeginPlay`
  ; Initialization
  (`|ExecutionSequence`))

(event `Delegate ReloadLevel`
  ; ReloadingLevel
  (bind _returnvalue (`GameplayStatics.GetCurrentLevelName` true))
  (`GameplayStatics.OpenLevel` (`KismetStringLibrary.Conv_StringToName` _returnvalue)))

(fn `UserConstructionScript`)