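; BP_Scoring is a score keeper that raises the score over time while active and reports it to the HUD.
; Initialization stores a HUD reference, which the author's note says is currently supplied by the Player.
; Activation starts a looping timer that increments Score every tenth of a second and passes the new value to the HUD.
; Deactivation clears that timer through its stored handle.
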(event `Delegate Initialize`
  (params (HUD :type "/Game/Blueprints/UI/WB_HUD Object Reference"))
  ;[0.15 0 0 0.5] Initialization (уже хороший метод, который можно вызывать в классе более высокого уровня или в Bootstrap - но пока он вызывается в Player)
  (set `self.HUD` HUD))

(event `Delegate Activate`
  ; Activation
  (bind _returnvalue (`KismetSystemLibrary.K2_SetTimerDelegate` (delegate `Delegate IncreaseScore`) 0.1 true))
  (set `self.ActivationTimerHandle` _returnvalue))

(event `Delegate IncreaseScore`
  ; Activation
  (bind _result (`/Engine/EditorBlueprintResources/StandardMacros.IncrementInt` (`self.Score`))
    (:`  `
      (bind _output_get (set `self.Score` _result))
      (`/Game/Blueprints/UI/WB_HUD.Delegate Update` (`self.HUD`) _output_get))))

(event `Delegate Deactivate`
  ; Deactivation
  (`KismetSystemLibrary.K2_ClearAndInvalidateTimerHandle` (`self.ActivationTimerHandle`)))

(fn `UserConstructionScript`)